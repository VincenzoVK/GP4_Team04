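; Base bomb actor that applies a randomized tweak to the player on overlap, then explodes and destroys itself.
; BeginPlay creates the tweak object from TweakType and tints the Niagara trails with TrailColour.
; BombFunction sends the tweak with a random Change percentage to BP_ThirdPersonCharacter and updates its camera distance.
; MakePlayerJump fakes blast knockback with a fixed upward impulse and horizontal push from the absolute offset, so always toward positive X/Y.
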(event `self.ReceiveBeginPlay`
  (bind _returnvalue (`|GenericCreateObject` (`self.TweakType`)))
  (set `self.Tweak` _returnvalue)
  (`NiagaraComponent.SetVariableLinearColor` (`self.Niagara_0`) "User.TrailColor" (`self.TrailColour`))
  (`NiagaraComponent.SetVariableLinearColor` (`self.Niagara5`) "User.TrailColor" (`self.TrailColour`))
  (`NiagaraComponent.SetVariableLinearColor` (`self.Niagara`) "User.TrailColor" (`self.TrailColour`))
  (`NiagaraComponent.SetVariableLinearColor` (`self.Niagara4`) "User.TrailColor" (`self.TrailColour`))
  (`NiagaraComponent.SetVariableLinearColor` (`self.Niagara1`) "User.TrailColor" (`self.TrailColour`))
  (`NiagaraComponent.SetVariableLinearColor` (`self.Niagara3`) "User.TrailColor" (`self.TrailColour`))
  (`NiagaraComponent.SetVariableLinearColor` (`self.Niagara2`) "User.TrailColor" (`self.TrailColour`)))

(event `MakePlayerJump`
  (bind _returnvalue (`GameplayStatics.GetPlayerCharacter` 0))
  (bind (_returnvalue_x _returnvalue_y) (`KismetMathLibrary.BreakVector` (* (`KismetMathLibrary.Vector_GetAbs` (- (`self.K2_GetActorLocation` _returnvalue) (`self.K2_GetActorLocation`))) (`self.ImpulseForce`))))
  ;[1 1 1] Make the player jump as if the bomb explodes
  (`CharacterMovementComponent.AddImpulse` (`Character.CharacterMovement` _returnvalue) (`KismetMathLibrary.MakeVector` _returnvalue_x _returnvalue_y 1000.0) true))

(event `BombFunction`
  (bind _tweak (`self.Tweak`))
  ;[1 1 1] Sizebomb
  (set `Tweak.PercentageType` "Change" _tweak)
  (set `Tweak.Percentage` (`KismetMathLibrary.RandomFloatInRange` 0.0 1.0) _tweak)
  (bind _asbp_third_person_character (cast `/Game/ThirdPerson/Blueprints/BP_ThirdPersonCharacter` (`GameplayStatics.GetPlayerCharacter` 0)))
  (`GP4Character.ReceiveTweak` _asbp_third_person_character _tweak)
  (`/Game/ThirdPerson/Blueprints/BP_ThirdPersonCharacter.ChangeCameraDistance` _asbp_third_person_character)
  (`self.MakePlayerJump`))

(event `self.ReceiveActorBeginOverlap`
  (params (OtherActor :type "Actor Object Reference"))
  ;[1 1 1] Overlap event for player
  (`/Engine/EditorBlueprintResources/StandardMacros.IsValid` OtherActor
    (:`Is Valid`
      (if (`self.ActorHasTag` OtherActor "Player")
        (`self.BombFunction`)
        (`NiagaraFunctionLibrary.SpawnSystemAtLocation` "/Game/LowPolyVFX/Particles/P_Ems_Explosion_03_Converted.P_Ems_Explosion_03_Converted" (`self.K2_GetActorLocation`) (struct) (2.0 2.0 2.0))
        (`self.K2_DestroyActor`)))))

(fn `UserConstructionScript`)