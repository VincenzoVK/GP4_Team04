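; Projectile that applies a randomized tweak to the character or tweakable object it hits.
; On BeginPlay it constructs its Tweak object from the TweakType class.
; On hit it sets that Tweak to a random percentage change and passes it to the target's ReceiveTweak.
; Character hits also change the camera distance and spawn an impact effect at the projectile's location.
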(event `self.ReceiveBeginPlay`
  (bind _returnvalue (`|GenericCreateObject` (`self.TweakType`)))
  (set `self.Tweak` _returnvalue))

(event `self.HandleHitObject`
  (params (HitActor :type "Actor Object Reference"))
  (bind _tweak (`self.Tweak`))
  ;[1 1 1] Apply Tweak on hit
  (set `Tweak.PercentageType` "Change" _tweak)
  (set `Tweak.Percentage` (`KismetMathLibrary.RandomFloatInRange` 0.0 1.0) _tweak)
  (bind _asbp_third_person_character (cast `/Game/ThirdPerson/Blueprints/BP_ThirdPersonCharacter` HitActor)
    (:`then`
      (`GP4Character.ReceiveTweak` _asbp_third_person_character _tweak)
      (`/Game/ThirdPerson/Blueprints/BP_ThirdPersonCharacter.ChangeCameraDistance` _asbp_third_person_character)
      (`NiagaraFunctionLibrary.SpawnSystemAtLocation` "/Game/LowPolyVFX/Particles/P_Hit_04_Converted.P_Hit_04_Converted" (`self.K2_GetActorLocation`) (struct) (2.5 2.5 2.5)))
    (:`CastFailed`
      (bind _astweakable_object (cast `TweakableObject` HitActor))
      (`TweakableObject.ReceiveTweak` _astweakable_object _tweak))))

(fn `UserConstructionScript`)