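; Base enemy character whose movement and AI state depend on its current size.
; On BeginPlay it binds to the player's size-check event and initializes its AI controller's Blackboard.
; HandleSizeChange writes the size to the Blackboard and sets walk speed and controller-yaw rotation, which is off only for Medium.
; It also spawns shrunken projectiles, reports hover to the player, toggles custom depth while tweaked, and mostly stubs the selection/tweak queries.
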(event `self.ReceiveBeginPlay`
  (bind _asgp4character (cast `GP4Character` (`GameplayStatics.GetPlayerCharacter` 0)))
  (add `GP4Character.OnCheckSizeChanged` _asgp4character (`|CreateDelegate` :!event `CheckSize`))
  (`self.InitializeEnemy`)
  (`self.HandleSizeChange`))

(event `self.OnChangeSize`
  (`self.HandleSizeChange`))

(event `self.OnStartHovered`
  (message `/Game/GP4_Blueprints/Widgets/BI_CrosshairInterface.ChangeColour` (`GameplayStatics.GetPlayerPawn` 0) true)
  (set `self.isHovered` true))

(event `self.OnStopHovered`
  (message `/Game/GP4_Blueprints/Widgets/BI_CrosshairInterface.ChangeColour` (`GameplayStatics.GetPlayerPawn` 0) false)
  (set `self.isHovered` false))

(event `self.OnShootProjectile`
  (params (ProjectileTransform :type "Transform Structure") (ProjectileClass :type "EnemyProjectile Class Reference"))
  (bind _returnvalue (`|SpawnActorFromClass` ProjectileClass ProjectileTransform "Undefined" "MultiplyWithRoot" null null))
  (`/Engine/EditorBlueprintResources/StandardMacros.IsValid` _returnvalue
    (:`Is Valid`
      (`self.SetActorScale3D` _returnvalue (0.2 0.2 0.2)))))

(event `self.StartTweaking`
  (`PrimitiveComponent.SetRenderCustomDepth` (`self.Mesh`) true))

(event `self.EndTweaking`
  (`PrimitiveComponent.SetRenderCustomDepth` (`self.Mesh`) false))

(fn `GetActiveTweak`
  (returns (Tweak :type "Tweak Object Reference"))
  (return null))

(fn `GetActiveTweakColor`
  (returns (color :type "Color Structure"))
  (return))

(fn `GetActiveTweakType`
  (returns (type :type "/Game/ThirdPerson/Blueprints/E_TweakAbilitySelector Enum"))
  (return "NewEnumerator0"))

(fn `GetPlayerSlefSelect`
  (returns (`playerselected?` :type Boolean))
  (return false))

(fn `GetSelectedObj`
  (returns (Items :type "Array of Actor Object Reference"))
  (return))

(fn `HandleSizeChange`
  (bind _charactermovement (`self.CharacterMovement`))
  (bind _currentsize (`self.CurrentSize`))
  (`BlackboardComponent.SetValueAsEnum` (`self.Blackboard`) (`KismetStringLibrary.Conv_StringToName` "SizeState") _currentsize)
  (switch `EEnemySizeState` _currentsize
    (:`Small`
      (set `CharacterMovementComponent.MaxWalkSpeed` (`self.SmallSizeWalkSpeed`) _charactermovement)
      (set `self.bUseControllerRotationYaw` true :!label _label))
    (:`Medium`
      (set `CharacterMovementComponent.MaxWalkSpeed` (`self.MediumSizeWalkSpeed`) _charactermovement)
      (set `self.bUseControllerRotationYaw` false))
    (:`Big`
      (set `CharacterMovementComponent.MaxWalkSpeed` (`self.BigSizeWalkSpeed`) _charactermovement)
      (goto _label))))

(fn `InitializeEnemy`
  (bind _asbase_enemy_aicontroller (cast `/Game/GP4_Blueprints/AI/BaseEnemyAIController` (`self.GetController`)))
  (bind _output_get (set `self.AIController` _asbase_enemy_aicontroller))
  (bind _output_get_2 (set `self.Blackboard` (`AIBlueprintHelperLibrary.GetBlackboard` _output_get)))
  (`BlackboardComponent.SetValueAsBool` _output_get_2 (`KismetStringLibrary.Conv_StringToName` "IsActive") true)
  (`BlackboardComponent.SetValueAsBool` _output_get_2 (`KismetStringLibrary.Conv_StringToName` "CanAttack") true)
  (`self.CheckSize`))

(fn `IsGOHovered`
  (returns (ReturnValue :type Boolean))
  (return (`self.isHovered`)))

(fn `isObjHovered?`
  (returns (`hovered?` :type Boolean))
  (return (`self.isHovered`)))

(fn `isObjSelected?`
  (returns (`selected?` :type Boolean))
  (return false))

(fn `isPlayerAiming?`
  (returns (isAiming :type Boolean))
  (return false))

(fn `UserConstructionScript`)