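; BP_ButtonDoor is a door that is destroyed once all the buttons in its ButtonsToPress array are pressed.
; Pressed and unpressed events raise and lower a counter, which each press compares against the array length.
; On a match it spawns a heavily scaled-up Niagara explosion, with no location specified, and destroys itself after a short delay.
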(event `/Game/GP4_Blueprints/ButtonSystem/BPI_ButtonSystemInterface.ButtonHasBeenPressed`
  (bind _result (`/Engine/EditorBlueprintResources/StandardMacros.IncrementInt` (`self.CounterOfButtonPressed`))
    (:`  `
      (if (== _result (`KismetArrayLibrary.Array_Length` (`self.ButtonsToPress`)))
        (`NiagaraFunctionLibrary.SpawnSystemAtLocation` "/Game/LowPolyVFX/Particles/P_Ems_Explosion_01_Converted.P_Ems_Explosion_01_Converted" (0.0 0.0 0.0) (struct) (100.0 100.0 100.0))
        (`KismetSystemLibrary.Delay` 1.0)
        (`self.K2_DestroyActor`)))))

(event `/Game/GP4_Blueprints/ButtonSystem/BPI_ButtonSystemInterface.ButtonHasBeenUnpressed`
  (`/Engine/EditorBlueprintResources/StandardMacros.DecrementInt` (`self.CounterOfButtonPressed`)))

(fn `UserConstructionScript`)