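; A trigger box actor that plays a one-time dialogue line when the player character overlaps it.
; On overlap it asks the game instance whether the message for its dialogue enum ID has been used.
; If not, it marks it used and passes the enum name to its dialogue component as a row name.
; A Debug flag shows the box in game.
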(event `self.ReceiveActorBeginOverlap`
  (params (OtherActor :type "Actor Object Reference"))
  (bind _id (`self.ID`))
  (bind _returnvalue (cast `/Game/GP4_Blueprints/Dialogue/BP_EnumDialogue` _id))
  (if (== OtherActor (`GameplayStatics.GetPlayerCharacter` 0))
    (bind _isused (message `/Game/GP4_Blueprints/Dialogue/DialogueManager_BPI.GetRowIndexUsed` (`GameplayStatics.GetGameInstance`) _returnvalue))
    (if (not _isused)
      (message `/Game/GP4_Blueprints/Dialogue/DialogueManager_BPI.SetRowIndexUsed` (`GameplayStatics.GetGameInstance`) _returnvalue)
      (`/Game/GP4_Blueprints/Dialogue/BP_DialogueComponent.OnDialogueTriggered` (`self.BP_DialogueComponent`) (`KismetStringLibrary.Conv_StringToName` (`|GetEnumeratorNameAsString` _id))))))

(fn `UserConstructionScript`
  (`SceneComponent.SetHiddenInGame` (`self.Box`) (not (`self.Debug`)) false))