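; Actor component that draws a screen-space targeting box around its owner while it is hovered or selected, tweak-targetable, and the player is aiming.
; BeginPlay creates a HUD widget for each component.
; Each tick it projects the eight collision-bounds corners to the screen, corrects for widget scale and takes their min/max.
; It sends that box, the pawn's active tweak name and color, and the selected state to the widget through interface messages.
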(event `self.ReceiveTick`
  (params (DeltaSeconds :type "Float (single-precision)"))
  (bind _returnvalue (`GameplayStatics.GetPlayerPawn` 0))
  (bind _screenspaceboundx (`self.ScreenspaceBoundX`))
  (bind _screenspaceboundy (`self.ScreenspaceBoundY`))
  (bind _boxstartsend_x (`KismetMathLibrary.BreakVector2D` (`self.BoxStartSend`)))
  (bind _screenspaceboundx_2 (`self.ScreenspaceBoundX`))
  (bind (_boxstartsend_x_2 _boxstartsend_y) (`KismetMathLibrary.BreakVector2D` (`self.BoxStartSend`)))
  (bind _screenspaceboundy_2 (`self.ScreenspaceBoundY`))
  (bind (_boxendsend_x _boxendsend_y) (`KismetMathLibrary.BreakVector2D` (`self.BoxEndSend`)))
  (bind _boxendsend_x_2 (`KismetMathLibrary.BreakVector2D` (`self.BoxEndSend`)))
  (bind _parent_actor (`self.Parent Actor`))
  ;[1 1 1] Convert 3D points to screenspace
  (bind _selected_ (message `/Game/GP4_Blueprints/EmmyTemp/BPI_TweakData.isObjSelected?` _parent_actor))
  (if _selected_
    (bind _isaiming (message `/Game/GP4_Blueprints/EmmyTemp/BPI_TweakData.isPlayerAiming?` (`GameplayStatics.GetPlayerPawn` 0) :!label _label))
    (if (and (`self.TweakTargettable`) _isaiming)
      (if true
        (bind (_c1pos _c2pos _c3pos _c4pos _c5pos _c6pos _c7pos _c8pos) (`self.Get Corners`))
        (bind _output_get (set `self.3DBounds` (`|MakeArray` _c1pos _c2pos _c3pos _c4pos _c5pos _c6pos _c7pos _c8pos)))
        (`self.Draw3DPointForDebug`)
        (bind _returnvalue_2 (`WidgetLayoutLibrary.GetPlayerScreenWidgetGeometry` (`GameplayStatics.GetPlayerController` 0)))
        (for (_array_element _array_index) _output_get
          (`KismetArrayLibrary.Array_Set` (`self.ScreenspaceBounds`) _array_index (* (`GameplayStatics.ProjectWorldToScreen` (`GameplayStatics.GetPlayerController` 0) _array_element) (/ (`SlateBlueprintLibrary.GetLocalSize` _returnvalue_2) (`SlateBlueprintLibrary.GetAbsoluteSize` _returnvalue_2))) true))
        (set `self.BoxStartSend` (9999999999.0 9999999999.0))
        (set `self.BoxEndSend` (0.0 0.0))
        ;[1 1 1] Find 2 Corners
        (for _array_element_2 (`self.ScreenspaceBounds`)
          (set `self.ScreenspaceBoundX` (`KismetMathLibrary.BreakVector2D` _array_element_2))
          (set `self.ScreenspaceBoundY` (`.Y` (`KismetMathLibrary.BreakVector2D` _array_element_2)))
          (set `self.BoxStartSend` (`KismetMathLibrary.MakeVector2D` (select `bool` (> _boxstartsend_x _screenspaceboundx_2) :`false` _boxstartsend_x :`true` _screenspaceboundx_2) (select `bool` (> _boxstartsend_y _screenspaceboundy_2) :`false` _boxstartsend_y :`true` _screenspaceboundy_2)))
          (set `self.BoxEndSend` (`KismetMathLibrary.MakeVector2D` (select `bool` (< _boxendsend_x_2 _screenspaceboundx) :`false` _boxendsend_x_2 :`true` _screenspaceboundx) (select `bool` (< _boxendsend_y _screenspaceboundy) :`false` _boxendsend_y :`true` _screenspaceboundy))))
        (bind _type (message `/Game/GP4_Blueprints/EmmyTemp/BPI_TweakData.GetActiveTweakType` _returnvalue))
        (bind _color (message `/Game/GP4_Blueprints/EmmyTemp/BPI_TweakData.GetActiveTweakColor` _returnvalue))
        (bind _selected__2 (message `/Game/GP4_Blueprints/EmmyTemp/BPI_TweakData.isObjSelected?` (`self.Parent Actor`)))
        (message `/Game/GP4_Blueprints/EmmyTemp/BPI_AimTargetInterface.SendBoxData` (`self.widgetRef`) (`self.BoxStartSend`) (`self.BoxEndSend`) (`|GetEnumeratorNameAsString` _type) _color _selected__2)))
    (else
      (bind _hovered_ (message `/Game/GP4_Blueprints/EmmyTemp/BPI_TweakData.isObjHovered?` _parent_actor))
      (if _hovered_
        (goto _label)))))

(event `Draw3DPointForDebug`)

(event `self.ReceiveBeginPlay`
  ;[1 1 1] Init
  (set `self.Parent Actor` (`self.GetOwner`))
  (bind _returnvalue (`|CreateWidget` "/Game/GP4_Blueprints/EmmyTemp/HUD.HUD_C" (`GameplayStatics.GetPlayerController` 0)))
  (set `self.widgetRef` _returnvalue)
  (`UserWidget.AddToViewport` _returnvalue 0))

(fn `Detect OnScreen`
  (params (CenterPos :type "Vector Structure"))
  (returns (screenPos :type "Vector2D Structure") (isOnScreen :type Boolean))
  ;[1 1 1] Detect if target is on screen
)

(fn `Get Corners`
  (returns (C1Pos :type "Vector Structure") (C2Pos :type "Vector Structure") (C3Pos :type "Vector Structure") (C4Pos :type "Vector Structure") (C5Pos :type "Vector Structure") (C6Pos :type "Vector Structure") (C7Pos :type "Vector Structure") (C8Pos :type "Vector Structure"))
  (locals (originVector :type "Vector Structure"))
  (bind (_origin _boxextent) (`Actor.GetActorBounds` (`self.GetOwner`) true false))
  (bind (_returnvalue_x _returnvalue_y _returnvalue_z) (`KismetMathLibrary.BreakVector` (* _boxextent (1.0 1.0 1.0))))
  ;[1 1 1] Get Corener
  (set `local.originVector` _origin)
  (set `self.x` _returnvalue_x)
  (set `self.y` _returnvalue_y)
  (set `self.z` _returnvalue_z)
  (return (+ (`KismetMathLibrary.MakeVector` (`self.x`) (`self.y`) (`self.z`)) (`local.originVector`)) (+ (`KismetMathLibrary.MakeVector` (* (`self.x`) -1.0) (`self.y`) (`self.z`)) (`local.originVector`)) (+ (`KismetMathLibrary.MakeVector` (`self.x`) (* (`self.y`) -1.0) (* (`self.z`) -1.0)) (`local.originVector`)) (+ (`KismetMathLibrary.MakeVector` (* (`self.x`) -1.0) (* (`self.y`) -1.0) (* (`self.z`) -1.0)) (`local.originVector`)) (+ (`KismetMathLibrary.MakeVector` (* (`self.x`) -1.0) (`self.y`) (* (`self.z`) -1.0)) (`local.originVector`)) (+ (`KismetMathLibrary.MakeVector` (`self.x`) (`self.y`) (* (`self.z`) -1.0)) (`local.originVector`)) (+ (`KismetMathLibrary.MakeVector` (* (`self.x`) -1.0) (* (`self.y`) -1.0) (`self.z`)) (`local.originVector`)) (+ (`KismetMathLibrary.MakeVector` (`self.x`) (* (`self.y`) -1.0) (`self.z`)) (`local.originVector`))))

(fn `GetActiveTweak`
  (returns (Tweak :type "Tweak Object Reference"))
  (return null))

(fn `GetActiveTweakColor`
  (returns (color :type "Color Structure"))
  (return))

(fn `GetActiveTweakType`
  (returns (type :type "/Game/ThirdPerson/Blueprints/E_TweakAbilitySelector Enum"))
  (return "NewEnumerator0"))

(fn `GetPlayerSlefSelect`
  (returns (`playerselected?` :type Boolean))
  (return false))

(fn `GetSelectedObj`
  (returns (Items :type "Array of Actor Object Reference"))
  (return))

(fn `GetWidgetRef`
  (returns (Widget :type "Object Object Reference"))
  (return null))

(fn `isObjHovered?`
  (returns (`hovered?` :type Boolean))
  (return false))

(fn `isObjSelected?`
  (returns (`selected?` :type Boolean))
  (return false))

(fn `isPlayerAiming?`
  (returns (isAiming :type Boolean))
  (return false))