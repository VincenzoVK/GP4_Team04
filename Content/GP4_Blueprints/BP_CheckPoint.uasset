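; Checkpoint actor that controls which streaming levels are loaded around it, using previous, current and next level name lists.
; LoadLevelbyName makes all three lists loaded and visible, blocking on load.
; UnLoadLevelbyName unloads and hides the PreviousLevels of the given character's PreviousCheckPoint, blocking on unload.
; ReloadLevelsCustom only repeats the unload logic, with its loop input unconnected, and overlap does nothing.
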(event `self.ReceiveBeginPlay`)

(event `self.LoadLevelByName`
  (`self.LoadLevelsCustom` (`self.PreviousLevels`))
  (`self.LoadLevelsCustom` (`self.CurrentLevels`))
  (`self.LoadLevelsCustom` (`self.NextLevels`)))

(event `self.UnLoadLevelByName`
  (params (Character :type "GP4Character Object Reference"))
  (`self.UnloadLevelsCustom` (`CheckPoint.PreviousLevels` (`GP4Character.PreviousCheckPoint` Character))))

(fn `LoadLevelsCustom`
  (params (Names :type "Array of Name"))
  (for _array_element Names
    (bind _returnvalue (`GameplayStatics.GetStreamingLevel` _array_element))
    (`/Engine/EditorBlueprintResources/StandardMacros.IsValid` _returnvalue
      (:`Is Valid`
        (set `LevelStreaming.bShouldBeLoaded` true _returnvalue)
        (set `LevelStreaming.bShouldBeVisible` true _returnvalue)
        (set `LevelStreaming.bShouldBlockOnLoad` true _returnvalue) ; either will work
      ))))

(fn `ReloadLevelsCustom`
  (params (Names :type "Array of Name"))
  (for _array_element _
    (bind _returnvalue (`GameplayStatics.GetStreamingLevel` _array_element))
    (`/Engine/EditorBlueprintResources/StandardMacros.IsValid` _returnvalue
      (:`Is Valid`
        (set `LevelStreaming.bShouldBeLoaded` false _returnvalue)
        (set `LevelStreaming.bShouldBeVisible` false _returnvalue)
        (set `LevelStreaming.bShouldBlockOnUnload` true _returnvalue)))))

(fn `UnloadLevelsCustom`
  (params (Names :type "Array of Name"))
  (for _array_element Names
    (bind _returnvalue (`GameplayStatics.GetStreamingLevel` _array_element))
    (`/Engine/EditorBlueprintResources/StandardMacros.IsValid` _returnvalue
      (:`Is Valid`
        (set `LevelStreaming.bShouldBeLoaded` false _returnvalue)
        (set `LevelStreaming.bShouldBeVisible` false _returnvalue)
        (set `LevelStreaming.bShouldBlockOnUnload` true _returnvalue)))))

(fn `UserConstructionScript`)