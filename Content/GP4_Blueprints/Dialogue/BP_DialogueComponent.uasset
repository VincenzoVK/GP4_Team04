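; Dialogue component that plays an NPC voice line with a matching subtitle when OnDialogueTriggered fires.
; It looks up the given row name in the NPCLines data table, then creates a WB_NarrativeWidget with the subtitle and a lifetime equal to the sound's duration, and plays the sound in 2D.
; A DoOnce with no reset limits it to one trigger, and debug prints show the duration or a missing row.
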(event `OnDialogueTriggered`
  (params (RowName :type Name))
  (`/Engine/EditorBlueprintResources/StandardMacros.DoOnce` false
    (:`Completed`
      (bind _returnvalue (`|GetDataTableRow` "/Game/GP4_Blueprints/Dialogue/NPCLines.NPCLines" RowName)
        (:`then`
          (bind _duration (`SoundBase.Duration` (`.SFX` (break `NarrativeInfo` _returnvalue))))
          (bind _output_get (set `self.LifeTime` _duration))
          (`KismetSystemLibrary.PrintString` (`KismetStringLibrary.Conv_DoubleToString` _duration) true true (struct :`G` 0.66 :`B` 1.0 :`A` 1.0) _duration)
          (bind _returnvalue_2 (`|CreateWidget` "/Game/GP4_Blueprints/Widgets/WB_NarrativeWidget.WB_NarrativeWidget_C" null _output_get (`KismetTextLibrary.Conv_StringToText` (`.Subtitle` (break `NarrativeInfo` _returnvalue)))))
          (bind _output_get_2 (set `self.Widget` _returnvalue_2))
          (`UserWidget.AddToViewport` _output_get_2 0)
          (`UserWidget.AddToViewport` _returnvalue_2 0)
          (`GameplayStatics.SpawnSound2D` (`.SFX` (break `NarrativeInfo` _returnvalue)) 1.0 1.0 0.0 null))
        (:`RowNotFound`
          (`KismetSystemLibrary.PrintString` "Couldnt find this dialogue entry in the table. Is the name on the sound trigger wrong?"))))))