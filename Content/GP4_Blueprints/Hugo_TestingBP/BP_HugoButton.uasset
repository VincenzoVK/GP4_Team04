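; BP_HugoButton is a toggle button that controls a connected lazer gate, in a testing folder.
; Each time an actor implementing the Tweakable interface begins overlapping its Trigger, it flips its Pressed state, swaps the button material between green and blue, and sends the matching pressed or unpressed message to the gate.
; GateDeactivated clears the gate reference, so later overlaps leave the button unchanged.
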(event `self.Trigger.OnComponentBeginOverlap`
  (params (OverlappedComponent :type "PrimitiveComponent Object Reference") (OtherActor :type "Actor Object Reference") (OtherComp :type "PrimitiveComponent Object Reference") (OtherBodyIndex :type Integer) (bFromSweep :type Boolean) (SweepResult :type "HitResult Structure (by ref)"))
  (if (`KismetSystemLibrary.DoesImplementInterface` OtherActor "/Script/GP4.Tweakable")
    (if (`self.Pressed`)
      (`/Engine/EditorBlueprintResources/StandardMacros.IsValid` (`self.ConnectedLazerGate`)
        (:`Is Valid`
          (message `/Game/GP4_Blueprints/Hugo_TestingBP/BI_HugoButtonSystem.HugoButtonUnPressed` (`self.ConnectedLazerGate`))
          (`PrimitiveComponent.SetMaterial` (`self.Button`) 0 "/Game/GP4_Materials/MI_Blue.MI_Blue")
          (set `self.Pressed` false)))
      (else
        (`/Engine/EditorBlueprintResources/StandardMacros.IsValid` (`self.ConnectedLazerGate`)
          (:`Is Valid`
            (`PrimitiveComponent.SetMaterial` (`self.Button`) 0 "/Game/GP4_Materials/MI_Green.MI_Green")
            (set `self.Pressed` true)
            (message `/Game/GP4_Blueprints/Hugo_TestingBP/BI_HugoButtonSystem.HugoButtonPressed` (`self.ConnectedLazerGate`))))))))

(event `/Game/GP4_Blueprints/Hugo_TestingBP/BI_HugoButtonSystem.GateDeactivated`
  (set `self.ConnectedLazerGate` null))

(fn `UserConstructionScript`)