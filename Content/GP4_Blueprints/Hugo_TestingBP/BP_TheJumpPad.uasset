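; BP_TheJumpPad is a jump pad that launches the player when BP_BoxyCharacter hits its Pad component.
; The hit event requires an exact class match, then calls LaunchCharacter on player 0's character rather than on the hitting actor.
; Launch velocity follows the Direction component's forward vector, multiplied per axis by the square of the Pad's world scale and a large constant, adding to existing velocity.
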(event `self.Pad.OnComponentHit`
  (params (HitComponent :type "PrimitiveComponent Object Reference") (OtherActor :type "Actor Object Reference") (OtherComp :type "PrimitiveComponent Object Reference") (NormalImpulse :type "Vector Structure") (Hit :type "HitResult Structure (by ref)"))
  (if (== (`GameplayStatics.GetObjectClass` OtherActor) "/Game/ThirdPerson/Blueprints/BP_BoxyCharacter.BP_BoxyCharacter_C")
    (`Character.LaunchCharacter` (`GameplayStatics.GetPlayerCharacter` 0) (* (`SceneComponent.GetForwardVector` (`self.direction`)) (* (`SceneComponent.K2_GetComponentScale` (`self.Pad`)) (* (`SceneComponent.K2_GetComponentScale` (`self.Pad`)) 15000.0))) false false)))

(fn `UserConstructionScript`)