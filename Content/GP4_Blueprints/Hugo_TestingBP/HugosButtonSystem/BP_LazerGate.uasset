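; BP_LazerGate is a laser gate that eliminates actors touching it until its linked buttons shut it off.
; Overlapping actors implementing BI_Eliminate get a hit effect and an eliminate message.
; Button press and release events maintain a count; when it equals the Buttons array length, the laser is destroyed for good and each button is notified.
; Tick prints the count, and an unused line trace remains.
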(event `self.Lazer.OnComponentBeginOverlap`
  (params (OverlappedComponent :type "PrimitiveComponent Object Reference") (OtherActor :type "Actor Object Reference") (OtherComp :type "PrimitiveComponent Object Reference") (OtherBodyIndex :type Integer) (bFromSweep :type Boolean) (SweepResult :type "HitResult Structure (by ref)"))
  (if (`KismetSystemLibrary.DoesImplementInterface` OtherActor "/Game/GP4_Blueprints/Hugo_TestingBP/BI_Eliminate.BI_Eliminate_C")
    (`NiagaraFunctionLibrary.SpawnSystemAtLocation` "/Game/LowPolyVFX/Particles/P_Ems_Hit_02_Converted.P_Ems_Hit_02_Converted" (`self.K2_GetActorLocation` OtherActor) (`KismetMathLibrary.Conv_VectorToRotator` (`SceneComponent.GetRightVector` (`self.DefaultSceneRoot`))) (* (`self.GetActorRelativeScale3D` OtherActor) 3.5))
    (message `/Game/GP4_Blueprints/Hugo_TestingBP/BI_Eliminate.Eliminate` OtherActor)))

(event `/Game/GP4_Blueprints/Hugo_TestingBP/BI_HugoButtonSystem.HugoButtonPressed`
  (if (not (`self.Deactivated`))
    (`/Engine/EditorBlueprintResources/StandardMacros.IncrementInt` (`self.ButtonsPressed`)
      (:`  `
        (if (== (`self.ButtonsPressed`) (`KismetArrayLibrary.Array_Length` (`self.Buttons`)))
          (`ActorComponent.K2_DestroyComponent` (`self.Lazer`))
          (for _array_element (`self.Buttons`)
            (message `/Game/GP4_Blueprints/Hugo_TestingBP/BI_HugoButtonSystem.GateDeactivated` _array_element)
            (set `self.Deactivated` true)))))))

(event `/Game/GP4_Blueprints/Hugo_TestingBP/BI_HugoButtonSystem.HugoButtonUnPressed`
  (`/Engine/EditorBlueprintResources/StandardMacros.DecrementInt` (`self.ButtonsPressed`)))

(event `self.ReceiveTick`
  (params (DeltaSeconds :type "Float (single-precision)"))
  (`KismetSystemLibrary.PrintString` (`KismetStringLibrary.Conv_IntToString` (`self.ButtonsPressed`))))

(fn `UserConstructionScript`)