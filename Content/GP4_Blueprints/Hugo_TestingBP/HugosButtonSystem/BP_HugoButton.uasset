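; BP_HugoButton is a trigger-volume button that controls an array of linked laser gates and a connected lamp.
; Overlaps from actors implementing the Tweakable interface send pressed or unpressed messages to each valid gate and the lamp, swapping the button material between emissive purple and blue.
; A GateDeactivated event forwards a deactivation message to the lamp.
; The Pressed variable and its reset branch are unused.
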(event `self.Trigger.OnComponentBeginOverlap`
  (params (OverlappedComponent :type "PrimitiveComponent Object Reference") (OtherActor :type "Actor Object Reference") (OtherComp :type "PrimitiveComponent Object Reference") (OtherBodyIndex :type Integer) (bFromSweep :type Boolean) (SweepResult :type "HitResult Structure (by ref)"))
  (if (`KismetSystemLibrary.DoesImplementInterface` OtherActor "/Script/GP4.Tweakable")
    (for _array_element (`self.ConnectedLazerGate`)
      (`/Engine/EditorBlueprintResources/StandardMacros.IsValid` _array_element
        (:`Is Valid`
          (`PrimitiveComponent.SetMaterial` (`self.Button`) 0 "/Game/GP4_Materials/MI_EmissivePurple.MI_EmissivePurple")
          (message `/Game/GP4_Blueprints/Hugo_TestingBP/BI_HugoButtonSystem.HugoButtonPressed` _array_element)
          (message `/Game/GP4_Blueprints/Hugo_TestingBP/BI_HugoButtonSystem.HugoButtonPressed` (`self.ConnectedLamp`)))))))

(event `/Game/GP4_Blueprints/Hugo_TestingBP/BI_HugoButtonSystem.GateDeactivated`
  (set `self.ConnectedLazerGate` (`self.ConnectedLazerGate`))
  (message `/Game/GP4_Blueprints/Hugo_TestingBP/BI_HugoButtonSystem.GateDeactivated` (`self.ConnectedLamp`)))

(event `self.Trigger.OnComponentEndOverlap`
  (params (OverlappedComponent :type "PrimitiveComponent Object Reference") (OtherActor :type "Actor Object Reference") (OtherComp :type "PrimitiveComponent Object Reference") (OtherBodyIndex :type Integer))
  (if (`KismetSystemLibrary.DoesImplementInterface` OtherActor "/Script/GP4.Tweakable")
    (for _array_element (`self.ConnectedLazerGate`)
      (`/Engine/EditorBlueprintResources/StandardMacros.IsValid` _array_element
        (:`Is Valid`
          (message `/Game/GP4_Blueprints/Hugo_TestingBP/BI_HugoButtonSystem.HugoButtonUnPressed` _array_element)
          (message `/Game/GP4_Blueprints/Hugo_TestingBP/BI_HugoButtonSystem.HugoButtonUnPressed` (`self.ConnectedLamp`))
          (`PrimitiveComponent.SetMaterial` (`self.Button`) 0 "/Game/GP4_Materials/MI_Blue.MI_Blue"))))))

(fn `UserConstructionScript`)