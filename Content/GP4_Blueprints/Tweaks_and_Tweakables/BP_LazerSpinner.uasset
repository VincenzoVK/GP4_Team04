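; BP_LazerSpinner is a laser hazard actor that eliminates actors touching either of its two trigger components.
; On overlap, each trigger checks the other actor for the BI_Eliminate interface, spawns a scaled Niagara hit effect at its location, then sends EliminateMessage.
; Both triggers run identical, duplicated logic, and the graph contains no spinning logic despite the asset's name.
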(event `self.lazertrigger1.OnComponentBeginOverlap`
  (params (OverlappedComponent :type "PrimitiveComponent Object Reference") (OtherActor :type "Actor Object Reference") (OtherComp :type "PrimitiveComponent Object Reference") (OtherBodyIndex :type Integer) (bFromSweep :type Boolean) (SweepResult :type "HitResult Structure (by ref)"))
  (if (`KismetSystemLibrary.DoesImplementInterface` OtherActor "/Game/GP4_Blueprints/Hugo_TestingBP/BI_Eliminate.BI_Eliminate_C")
    (`NiagaraFunctionLibrary.SpawnSystemAtLocation` "/Game/LowPolyVFX/Particles/P_Ems_Hit_02_Converted.P_Ems_Hit_02_Converted" (`self.K2_GetActorLocation` OtherActor) (struct) (* (`self.GetActorScale3D` OtherActor) 3.5))
    (message `/Game/GP4_Blueprints/Hugo_TestingBP/BI_Eliminate.Eliminate` OtherActor)))

(event `self.lazertrigger.OnComponentBeginOverlap`
  (params (OverlappedComponent :type "PrimitiveComponent Object Reference") (OtherActor :type "Actor Object Reference") (OtherComp :type "PrimitiveComponent Object Reference") (OtherBodyIndex :type Integer) (bFromSweep :type Boolean) (SweepResult :type "HitResult Structure (by ref)"))
  (if (`KismetSystemLibrary.DoesImplementInterface` OtherActor "/Game/GP4_Blueprints/Hugo_TestingBP/BI_Eliminate.BI_Eliminate_C")
    (`NiagaraFunctionLibrary.SpawnSystemAtLocation` "/Game/LowPolyVFX/Particles/P_Ems_Hit_02_Converted.P_Ems_Hit_02_Converted" (`self.K2_GetActorLocation` OtherActor) (struct) (* (`self.GetActorScale3D` OtherActor) 3.5))
    (message `/Game/GP4_Blueprints/Hugo_TestingBP/BI_Eliminate.Eliminate` OtherActor)))

(fn `UserConstructionScript`
  (`parent.UserConstructionScript`))