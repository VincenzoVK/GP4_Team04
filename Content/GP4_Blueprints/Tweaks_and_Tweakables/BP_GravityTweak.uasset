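; Gravity tweak that sets a tweakable object's gravity scale by lerping between a min and max scale using a percentage.
; It targets the object's CharacterMovementComponent first, falling back to a GravityComponent.
; When a character's resulting scale is zero or below, it adds a tiny upward force.
; It also reports the current scale as a normalized percentage and exposes the min and max values.
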(event `self.OnApplyTweak`
  (params (TweakableObject :type "Actor Object Reference"))
  (bind _returnvalue (`Actor.GetComponentByClass` TweakableObject "/Script/Engine.CharacterMovementComponent"))
  (bind _returnvalue_2 (`Actor.GetComponentByClass` TweakableObject "/Script/GP4.GravityComponent"))
  (bind _returnvalue_3 (`KismetMathLibrary.Lerp` (`self.Min Scale`) (`self.Max Scale`) (`self.Percentage`)))
  (`/Engine/EditorBlueprintResources/StandardMacros.IsValid` _returnvalue
    (:`Is Valid`
      (set `CharacterMovementComponent.GravityScale` _returnvalue_3 _returnvalue)
      (if (<= _returnvalue_3 0.0)
        (`CharacterMovementComponent.AddForce` _returnvalue (0.0 0.0 1.0))))
    (:`Is Not Valid`
      (`/Engine/EditorBlueprintResources/StandardMacros.IsValid` _returnvalue_2
        (:`Is Valid`
          (set `GravityComponent.GravityScale` _returnvalue_3 _returnvalue_2))))))

(fn `GetCurrentPercentage`
  (params (TweakableObject :type "Actor Object Reference"))
  (returns (ReturnValue :type "Float (single-precision)"))
  (bind _returnvalue (`Actor.GetComponentByClass` TweakableObject "/Script/Engine.CharacterMovementComponent"))
  (bind _returnvalue_2 (`Actor.GetComponentByClass` TweakableObject "/Script/GP4.GravityComponent"))
  (`/Engine/EditorBlueprintResources/StandardMacros.IsValid` _returnvalue
    (:`Is Valid`
      (return (`KismetMathLibrary.NormalizeToRange` (`CharacterMovementComponent.GravityScale` _returnvalue) (`self.Min Scale`) (`self.Max Scale`))))
    (:`Is Not Valid`
      (`/Engine/EditorBlueprintResources/StandardMacros.IsValid` _returnvalue_2
        (:`Is Valid`
          (return (`KismetMathLibrary.NormalizeToRange` (`GravityComponent.GravityScale` _returnvalue_2) (`self.Min Scale`) (`self.Max Scale`))))))))

(fn `GetMaxValue`
  (returns (ReturnValue :type "Float (single-precision)"))
  (return (`self.Max Scale`)))

(fn `GetMinValue`
  (returns (ReturnValue :type "Float (single-precision)"))
  (return (`self.Min Scale`)))