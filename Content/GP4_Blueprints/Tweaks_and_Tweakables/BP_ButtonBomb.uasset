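; BP_ButtonBomb is a bomb that turns red and explodes after a countdown when a Tweakable actor overlaps its box.
; EliminatewithRule triggers the same blast after a short delay.
; Detonation sphere-traces around the mesh, eliminates BI_Eliminate actors with Niagara effects, then destroys the bomb.
; A Growth event loops a timeline to keep enlarging the mesh, which also scales blast radius and effect size.
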(event `Growth`
  (bind _mesh (`self.Mesh`))
  (`Timeline|Grow` :!via `PlayFromStart` :!label _label
    (:`Finished`
      (`SceneComponent.SetRelativeScale3D` _mesh (+ (`SceneComponent.RelativeScale3D` _mesh) (0.1 0.1 0.1)))
      (goto _label :!via `PlayFromStart`))))

(event `self.Box.OnComponentBeginOverlap`
  (params (OverlappedComponent :type "PrimitiveComponent Object Reference") (OtherActor :type "Actor Object Reference") (OtherComp :type "PrimitiveComponent Object Reference") (OtherBodyIndex :type Integer) (bFromSweep :type Boolean) (SweepResult :type "HitResult Structure (by ref)"))
  (if (`KismetSystemLibrary.DoesImplementInterface` OtherActor "/Script/GP4.Tweakable")
    (`self.DetonateCountdown`)))

(event `DetonateCountdown`
  (`PrimitiveComponent.SetMaterial` (`self.Mesh`) 0 "/Game/GP4_Materials/MI_Red.MI_Red")
  (`Timeline|CountDown`
    (:`Finished`
      (`self.Detonate`))))

(event `Detonate`
  (bind _mesh (`self.Mesh`))
  (bind _mesh_2 (`self.Mesh`))
  (bind _relativelocation (`SceneComponent.RelativeLocation` _mesh))
  (bind _outhits (`KismetSystemLibrary.SphereTraceMulti` _relativelocation _relativelocation (`KismetMathLibrary.VSize` (* (`SceneComponent.RelativeScale3D` _mesh) 110.0)) "TraceTypeQuery1"))
  (`NiagaraFunctionLibrary.SpawnSystemAtLocation` "/Game/LowPolyVFX/Particles/P_Explosion_02_Converted.P_Explosion_02_Converted" (`SceneComponent.RelativeLocation` _mesh_2) (struct) (* (`SceneComponent.RelativeScale3D` _mesh_2) 10.0))
  (for _array_element _outhits
    (bind (_bblockinghit _binitialoverlap _time _distance _location _impactpoint _normal _impactnormal _physmat _hitactor) (`GameplayStatics.BreakHitResult` _array_element))
    (if (`KismetSystemLibrary.DoesImplementInterface` _hitactor "/Game/GP4_Blueprints/Hugo_TestingBP/BI_Eliminate.BI_Eliminate_C")
      (`NiagaraFunctionLibrary.SpawnSystemAtLocation` "/Game/LowPolyVFX/Particles/P_Ems_Explosion_01_Converted.P_Ems_Explosion_01_Converted" (`self.K2_GetActorLocation` _hitactor) (struct) (* (`self.GetActorScale3D` _hitactor) 5.0))
      (message `/Game/GP4_Blueprints/Hugo_TestingBP/BI_Eliminate.Eliminate` _hitactor)))
  (`self.K2_DestroyActor`))

(event `/Game/GP4_Blueprints/Hugo_TestingBP/BI_Eliminate.EliminateWithRule`
  (`PrimitiveComponent.SetMaterial` (`self.Mesh`) 0 "/Game/GP4_Materials/MI_Red.MI_Red")
  (`KismetSystemLibrary.Delay` 0.8)
  (`self.Detonate`))

(fn `UserConstructionScript`
  (`parent.UserConstructionScript`))