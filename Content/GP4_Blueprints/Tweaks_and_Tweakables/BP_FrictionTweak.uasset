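; Friction tweak that maps a percentage onto the slipperiness of a target object in the tweakables system.
; Targets with a CharacterMovementComponent get ground friction and walking braking deceleration lerped by the percentage, while max walk speed uses the inverse percentage.
; Other targets are cast to TweakableObject and receive the lerped value through SetFriction.
; Getters expose the friction range and normalize the target's current friction back to a percentage.
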(event `self.OnApplyTweak`
  (params (TweakableObject :type "Actor Object Reference"))
  (bind _returnvalue (`Actor.GetComponentByClass` TweakableObject "/Script/Engine.CharacterMovementComponent"))
  (bind _returnvalue_2 (`KismetMathLibrary.Lerp` (`self.MinScale`) (`self.MaxScale`) (`self.Percentage`)))
  (`/Engine/EditorBlueprintResources/StandardMacros.IsValid` _returnvalue
    (:`Is Valid`
      (set `CharacterMovementComponent.GroundFriction` _returnvalue_2 _returnvalue)
      (set `CharacterMovementComponent.BrakingDecelerationWalking` (`KismetMathLibrary.Lerp` (`self.MinBrakingScale`) (`self.MaxBreakingScale`) (`self.Percentage`)) _returnvalue)
      (set `CharacterMovementComponent.MaxWalkSpeed` (`KismetMathLibrary.Lerp` (`self.MinWalkingScale`) (`self.MaxWalkingScale`) (- 1.0 (`self.Percentage`))) _returnvalue))
    (:`Is Not Valid`
      (bind _astweakable_object (cast `TweakableObject` TweakableObject))
      (`TweakableObject.SetFriction` _astweakable_object _returnvalue_2)
      (`/Engine/EditorBlueprintResources/StandardMacros.IsValid` (`Actor.GetComponentByClass` _astweakable_object "/Script/Engine.StaticMeshComponent")))))

(fn `GetCurrentPercentage`
  (params (TweakableObject :type "Actor Object Reference"))
  (returns (ReturnValue :type "Float (single-precision)"))
  (bind _returnvalue (`Actor.GetComponentByClass` TweakableObject "/Script/Engine.CharacterMovementComponent"))
  (`/Engine/EditorBlueprintResources/StandardMacros.IsValid` _returnvalue
    (:`Is Valid`
      (return (`KismetMathLibrary.NormalizeToRange` (`CharacterMovementComponent.GroundFriction` _returnvalue) (`self.MinScale`) (`self.MaxScale`))))
    (:`Is Not Valid`
      (bind _astweakable_object (cast `TweakableObject` TweakableObject))
      (bind _returnvalue_2 (`TweakableObject.GetFriction` _astweakable_object))
      (return (`KismetMathLibrary.NormalizeToRange` _returnvalue_2 (`self.MinScale`) (`self.MaxScale`))))))

(fn `GetMaxValue`
  (returns (ReturnValue :type "Float (single-precision)"))
  (return (`self.MaxScale`)))

(fn `GetMinValue`
  (returns (ReturnValue :type "Float (single-precision)"))
  (return (`self.MinScale`)))