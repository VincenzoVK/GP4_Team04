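; BP_Multiplier is an actor that grows over time and duplicates itself until the third-person character touches it.
; A looping timeline enlarges the mesh in steps; at SizeTrigger it turns red and starts a second timeline.
; When that ends, it spawns another BP_Multiplier at its location, resets to its original size and white material, and restarts.
; Character overlap turns it blue and sets Deactivated, which blocks further growth cycles and spawning.
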(event `self.ReceiveBeginPlay`
  (`self.TheLoop`)
  (set `self.OriginalSize` (`SceneComponent.RelativeScale3D` (`self.Mesh`))))

(event `TheLoop`
  (bind _mesh (`self.Mesh`))
  (bind _relativescale3d_x (`KismetMathLibrary.BreakVector` (`SceneComponent.RelativeScale3D` (`self.Mesh`))))
  (if (not (`self.Deactivated`))
    (`Timeline|Timeline` :!via `PlayFromStart` :!label _label
      (:`Finished`
        (`SceneComponent.SetRelativeScale3D` _mesh (+ (`SceneComponent.RelativeScale3D` _mesh) (0.1 0.1 0.1)))
        (if (>= _relativescale3d_x (`self.SizeTrigger`))
          (`self.Detonating`)
          (elif (not (`self.Deactivated`))
            (goto _label :!via `PlayFromStart`)))))))

(event `Detonating`
  (bind _mesh (`self.Mesh`))
  (bind _relativescale3d_x (`KismetMathLibrary.BreakVector` (`SceneComponent.RelativeScale3D` (`self.Mesh`))))
  (if (not (`self.Deactivated`))
    (`PrimitiveComponent.SetMaterial` (`self.Mesh`) 0 "/Game/GP4_Materials/MI_Red.MI_Red")
    (`Timeline|Timeline_0` :!via `PlayFromStart`
      (:`Finished`
        (if (>= _relativescale3d_x (`self.SizeTrigger`))
          (if (not (`self.Deactivated`))
            (`|SpawnActorFromClass` "BP_Multiplier_C" (`KismetMathLibrary.Conv_VectorToTransform` (`SceneComponent.K2_GetComponentLocation` _mesh)) "Undefined" "MultiplyWithRoot" null null)
            (`KismetSystemLibrary.PrintString` "BANG")
            (`SceneComponent.SetRelativeScale3D` _mesh (`self.OriginalSize`))
            (`PrimitiveComponent.SetMaterial` (`self.Mesh`) 0 "/Game/GP4_Materials/MI_White.MI_White" :!label _label_2)
            (`self.TheLoop`))
          (else
            (goto _label_2)))))))

(event `self.collision.OnComponentBeginOverlap`
  (params (OverlappedComponent :type "PrimitiveComponent Object Reference") (OtherActor :type "Actor Object Reference") (OtherComp :type "PrimitiveComponent Object Reference") (OtherBodyIndex :type Integer) (bFromSweep :type Boolean) (SweepResult :type "HitResult Structure (by ref)"))
  (if (== (`GameplayStatics.GetObjectClass` OtherActor) "/Game/ThirdPerson/Blueprints/BP_ThirdPersonCharacter.BP_ThirdPersonCharacter_C")
    (if (not (`self.Deactivated`))
      (`PrimitiveComponent.SetMaterial` (`self.Mesh`) 0 "/Game/GP4_Materials/MI_Blue.MI_Blue")
      (set `self.Deactivated` true))))

(fn `UserConstructionScript`
  (`parent.UserConstructionScript`))