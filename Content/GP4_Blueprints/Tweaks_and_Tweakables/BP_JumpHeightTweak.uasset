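; A tweak Blueprint that adjusts how high a Character jumps by changing its movement component's JumpZVelocity.
; Applying the tweak sets that velocity by interpolating between MinHeight and MaxHeight using Percentage.
; GetCurrentPercentage does the inverse, normalizing the Character's current velocity to the same range, and both paths act only on Character targets.
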(event `self.OnApplyTweak`
  (params (TweakableObject :type "Actor Object Reference"))
  (bind _ascharacter (cast `Character` TweakableObject))
  (set `CharacterMovementComponent.JumpZVelocity` (`KismetMathLibrary.Lerp` (`self.MinHeight`) (`self.MaxHeight`) (`self.Percentage`)) (`Character.CharacterMovement` _ascharacter)))

(fn `GetCurrentPercentage`
  (params (TweakableObject :type "Actor Object Reference"))
  (returns (ReturnValue :type "Float (single-precision)"))
  (bind _ascharacter (cast `Character` TweakableObject))
  (return (`KismetMathLibrary.NormalizeToRange` (`CharacterMovementComponent.JumpZVelocity` (`Character.CharacterMovement` _ascharacter)) (`self.MinHeight`) (`self.MaxHeight`))))