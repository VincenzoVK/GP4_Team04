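; Spawner actor that places one randomly chosen object from its PossibleObjects list at its own location when play begins.
; The spawned actor gets a random rotation on all three axes and a random uniform scale multiplier between MinimumSize and MaximumSize, applied on top of the spawner's scale.
; Spawning adjusts for collisions where possible but always succeeds, and the construction script is empty.
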(event `self.ReceiveBeginPlay`
  (bind (_returnvalue_location _returnvalue_rotation _returnvalue_scale) (`KismetMathLibrary.BreakTransform` (`self.GetTransform`)))
  (`|SpawnActorFromClass` (`KismetArrayLibrary.Array_Random` (`self.PossibleObjects`)) (`KismetMathLibrary.MakeTransform` _returnvalue_location (`KismetMathLibrary.MakeRotator` (`KismetMathLibrary.RandomFloatInRange` 1.0 360.0) (`KismetMathLibrary.RandomFloatInRange` 1.0 360.0) (`KismetMathLibrary.RandomFloatInRange` 1.0 360.0)) (* _returnvalue_scale (`KismetMathLibrary.RandomFloatInRange` (`self.MinimumSize`) (`self.MaximumSize`)))) "AdjustIfPossibleButAlwaysSpawn" "MultiplyWithRoot" null null))

(fn `UserConstructionScript`)