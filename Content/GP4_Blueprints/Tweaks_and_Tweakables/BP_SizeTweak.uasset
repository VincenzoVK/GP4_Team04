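; BP_SizeTweak is a tweak that changes the size of a tweakable object.
; Applying it sets a uniform actor scale by interpolating between MinScale and MaxScale with a percentage.
; It reads the current percentage back by normalizing the object's X scale over that same range, and exposes both bounds through getters.
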(event `self.OnApplyTweak`
  (params (TweakableObject :type "Actor Object Reference"))
  (`Actor.SetActorScale3D` TweakableObject (`KismetMathLibrary.Conv_DoubleToVector` (`KismetMathLibrary.Lerp` (`self.MinScale`) (`self.MaxScale`) (`self.Percentage`)))))

(fn `GetCurrentPercentage`
  (params (TweakableObject :type "Actor Object Reference"))
  (returns (ReturnValue :type "Float (single-precision)"))
  (bind _returnvalue_x (`KismetMathLibrary.BreakVector` (`Actor.GetActorScale3D` TweakableObject)))
  (return (`KismetMathLibrary.NormalizeToRange` _returnvalue_x (`self.MinScale`) (`self.MaxScale`))))

(fn `GetMaxValue`
  (returns (ReturnValue :type "Float (single-precision)"))
  (return (`self.MaxScale`)))

(fn `GetMinValue`
  (returns (ReturnValue :type "Float (single-precision)"))
  (return (`self.MinScale`)))