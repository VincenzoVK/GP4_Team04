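; A tutorial trigger Blueprint that shows a text message while the player character stands inside its trigger volume.
; On BeginPlay it passes InputText to the TEXT component's widget and hides that component.
; Begin and end overlap events on Trigger toggle the text's visibility, responding only to actors whose class is exactly BP_BoxyCharacter.
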(event `self.ReceiveBeginPlay`
  ;[1 1 1] Init
  (message `/Game/GP4_Blueprints/Widgets/BI_DisplayText.SetDisplayText` (`WidgetComponent.GetWidget` (`self.TEXT`)) (`self.InputText`))
  (`SceneComponent.SetVisibility` (`self.TEXT`) false false))

(event `self.Trigger.OnComponentBeginOverlap`
  (params (OverlappedComponent :type "PrimitiveComponent Object Reference") (OtherActor :type "Actor Object Reference") (OtherComp :type "PrimitiveComponent Object Reference") (OtherBodyIndex :type Integer) (bFromSweep :type Boolean) (SweepResult :type "HitResult Structure (by ref)"))
  ;[1 1 1] Trigger
  (if (== (`GameplayStatics.GetObjectClass` OtherActor) "/Game/ThirdPerson/Blueprints/BP_BoxyCharacter.BP_BoxyCharacter_C")
    (`SceneComponent.SetVisibility` (`self.TEXT`) true false)))

(event `self.Trigger.OnComponentEndOverlap`
  (params (OverlappedComponent :type "PrimitiveComponent Object Reference") (OtherActor :type "Actor Object Reference") (OtherComp :type "PrimitiveComponent Object Reference") (OtherBodyIndex :type Integer))
  ;[1 1 1] Trigger
  (if (== (`GameplayStatics.GetObjectClass` OtherActor) "/Game/ThirdPerson/Blueprints/BP_BoxyCharacter.BP_BoxyCharacter_C")
    (`SceneComponent.SetVisibility` (`self.TEXT`) false false)))

(fn `UserConstructionScript`)